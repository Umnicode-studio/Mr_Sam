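; Main menu actor that makes a point light's brightness drift randomly and smoothly.
; A timeline lerps intensity from the last value to a target; when it finishes, Tick restarts it via a flag.
; Each new target is a random step from the current intensity, clamped between a hard-coded floor and MaxLightValue.
; An unconnected chain for a level transit widget with looping loading video never runs.
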(event `self.ReceiveBeginPlay`
  (set `self.RestartTimeline` true))

(event `self.ReceiveTick`
  (params (DeltaSeconds :type "Float (single-precision)"))
  (if (`self.RestartTimeline`)
    (set `self.RestartTimeline` false)
    ;[1 1 1] Smooth change of light strength
    (bind (_direction _progress) (`Timeline|Timeline` :`NewTime` (`self.Delay`) :!via `PlayFromStart`)
      (:`Update`
        (`LightComponent.SetIntensity` (`self.PointLight`) (`KismetMathLibrary.Lerp` (`self.LastIntensity`) (`self.TargetIntensity`) _progress)))
      (:`Finished`
        (set `self.RestartTimeline` true)
        (`self.UpdateTargetIntensity`)))))

(fn `UpdateTargetIntensity`
  (bind _step (`self.Step`))
  (bind _intensity (`LightComponentBase.Intensity` (`self.PointLight`)))
  ;[1 1 1] Random light value
  (set `self.LastIntensity` _intensity)
  (set `self.TargetIntensity` (`KismetMathLibrary.RandomFloatInRange` (`KismetMathLibrary.FMax` 50000.0 (- _intensity _step)) (`KismetMathLibrary.FMin` (`self.MaxLightValue`) (+ _step _intensity)))))

(fn `UserConstructionScript`)